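; BP_Tank is a player-controllable tank pawn with turret aiming, track-based movement, firing and a health bar.
; BeginPlay wires barrel and turret into TankAiming, both tracks into TankMovement, and passes itself to the BP_Healthbar widget.
; Input axes rotate the azimuth gimbal and spring arm for camera aim and send movement intents to TankMovement.
; Actions fire through TankAiming and toggle between first- and third-person cameras.
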(event EventBeginPlay
  ;[1 1 1] Initialises aiming and movement component and Healthbar
  (Class|TankAimingComponent|Initialise (Variables|Default|GetTankAiming) (Variables|Default|GetBarrel) (Variables|Default|GetTurret))
  (Class|TankMovementComponent|Initialise (Variables|Default|GetTankMovement) (Variables|Default|GetLeft%20Track) (Variables|Default|GetRight%20Track))
  (CallFunction|InitialiseHealthBarWidget self))

(event Input|ActionEvents|InputActionFire
  (params (Key :type Key%20Structure))
  ;[1 1 1] Weapon Input Binding
  ;;[1 1 1] Fire method
  (:Pressed
    (Class|TankAimingComponent|Fire (Variables|Default|GetTankAiming))))

(event Input|ActionEvents|InputActionSwapCam
  (params (Key :type Key%20Structure))
  ;[1 1 1] Camera swapping
  (:Pressed
    (Components|Activation|ToggleActive (Variables|Default|Get1st%20Person))
    (Components|Activation|ToggleActive (Variables|Default|Get3rd%20Person))))

(event Input|AxisEvents|InputAxisAimAzimuth/Horizontal
  (params (AxisValue :type Float%20%28single-precision%29))
  ;[1 1 1] Weapon Input Binding
  (Transformation|AddLocalRotation (Variables|Default|GetAzimuth/Horizontal%20Gimbal) (Math|Rotator|MakeRotator 0.0 0.0 AxisValue) false false))

(event Input|AxisEvents|InputAxisMoveForward
  (params (AxisValue :type Float%20%28single-precision%29))
  ;[1 1 1] Tank Movement Binding
  (Class|TankMovementComponent|IntendMoveForward (Variables|Default|GetTankMovement) AxisValue))

(event Input|AxisEvents|InputAxisAimElavation/Vertical
  (params (AxisValue :type Float%20%28single-precision%29))
  ;[1 1 1] Weapon Input Binding
  (Transformation|AddLocalRotation (Variables|Default|GetSpringArm) (Math|Rotator|MakeRotator 0.0 AxisValue 0.0) false false))

(event Input|AxisEvents|InputAxisTurnRight
  (params (AxisValue :type Float%20%28single-precision%29))
  ;[1 1 1] Tank Movement Binding
  (Class|TankMovementComponent|IntendTurnRight (Variables|Default|GetTankMovement) AxisValue))

(fn ConstructionScript)

(fn InitialiseHealthBarWidget
  (bind _asbp_healthbar (Utilities|Casting|CastToBP_Healthbar (UserInterface|GetUserWidgetObject (Variables|Default|GetWidget))))
  (Variables|/Game/BluePrints/UI/BP_Healthbar.BP_Healthbar_C|SetMy%20Tank _asbp_healthbar self)
  (return))